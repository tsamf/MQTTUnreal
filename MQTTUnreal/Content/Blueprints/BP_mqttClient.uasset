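; MQTT client actor that bridges broker messages to the BP_EdgeDevice actors in the level.
; On BeginPlay it creates the client, binds its handlers, requests a connection with blank credentials, then maps each device by Topic and subscribes without waiting for the connect callback.
; Incoming messages are passed to the matching device's RecieveMessage by topic lookup, with debug prints for message, publish and subscription events.
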(event Custom|OnPublishCallback
  (params (mid :type Integer))
  (Development|PrintString (Utilities|String|Append "Message published: Mid: " (Utilities|String|ToString(Integer) mid)) true true "(R=0.327744,G=1.000000,B=0.139947,A=1.000000)" 1e+01))

(event Custom|OnSubscriberCallback
  (params (mid :type Integer) (qos :type Array%20of%20Integers))
  (Development|PrintString (Utilities|String|Append "Subscribed! Mid: " (Utilities|String|ToString(Integer) mid)) true true "(R=0.327744,G=1.000000,B=0.139947,A=1.000000)" 1e+01))

(event Custom|OnUnsubscribedCallBack
  (params (mid :type Integer))
  (Development|PrintString (Utilities|String|Append "Unsubscribed! Mid: " (Utilities|String|ToString(Integer) mid)) true true "(R=0.327744,G=1.000000,B=0.139947,A=1.000000)" 1e+01))

(event Custom|OnMessageCallback
  (params (message :type Mqtt%20Message%20Structure))
  (bind (_message _messagebuffer _topic) (Utilities|Struct|BreakMqttMessage message))
  (Development|PrintString (Utilities|String|Append _topic _message))
  (Default|RecieveMessage (.Value (Utilities|Map|Find (Variables|Default|GetEdgeDevices) _topic)) _message))

(event Custom|OnErrorCallback
  (params (code :type Integer) (message :type String)))

(event Custom|OnConnectCallback)

(event EventBeginPlay
  (Utilities|FlowControl|Sequence
    (:then_0
      (bind _returnvalue (Class|MqttUtilitiesBPL|CreateMqttClient (Variables|Default|GetMqttClientConfiguration)))
      (Variables|Default|SetMqttClientInterface _returnvalue)
      (Class|MqttClientInterface|SetonPublishHandler (Variables|Default|GetMqttClientInterface) (delegate Custom|OnPublishCallback))
      (Class|MqttClientInterface|SetonSubscribeHandler (Variables|Default|GetMqttClientInterface) (delegate Custom|OnSubscriberCallback))
      (Class|MqttClientInterface|SetonUnsubscribeHandler (Variables|Default|GetMqttClientInterface) (delegate Custom|OnUnsubscribedCallBack))
      (Class|MqttClientInterface|SetonMessageHandler (Variables|Default|GetMqttClientInterface) (delegate Custom|OnMessageCallback))
      (Class|MqttClientInterface|SetonErrorHandler (Variables|Default|GetMqttClientInterface) (delegate Custom|OnErrorCallback))
      (Development|PrintString (Utilities|String|Append "Error - Code: " (Utilities|String|ToString(Integer) (stale Custom|OnErrorCallback code)) " Message: " (stale Custom|OnErrorCallback message))))
    (:then_1
      (Class|MqttClientInterface|Connect (Variables|Default|GetMqttClientInterface) (Utilities|Struct|MakeMqttConnectionData) (delegate Custom|OnConnectCallback)))
    (:then_2
      (bind _outactors (Actor|GetAllActorsOfClass "/Game/Blueprints/BP_EdgeDevice.BP_EdgeDevice_C"))
      (for _array_element _outactors
        (Utilities|Map|Add (Variables|Default|GetEdgeDevices) (Variables|/Game/Blueprints/BP_EdgeDevice.BP_EdgeDevice_C|GetTopic _array_element) _array_element)
        (Class|MqttClientInterface|Subscribe (Variables|Default|GetMqttClientInterface) (Variables|/Game/Blueprints/BP_EdgeDevice.BP_EdgeDevice_C|GetTopic _array_element))))))

(fn ConstructionScript)